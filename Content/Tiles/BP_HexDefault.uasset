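; BP_HexDefault is a hex grid tile on which the player can place one tower.
; Hovering swaps the mesh material to blue and restores the base material cached at BeginPlay.
; Interacting spawns the supplied tower class at TowerSpawnLocation, guarded by IsTowerSpawned.
; It also fires a debug shout that prints ring, number and side, and spawns BP_PathNewDefault at world origin for the Origin-tagged tile.
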(event Custom|Event_Shout
  ;[0.8261 0.5739 0.15 0.5] Debug event to check the interaction system works
  (Development|PrintString (Utilities|String|Append "Ring: " (Utilities|String|ToString(Integer) (Variables|Default|GetRing)) " | Number: " (Utilities|String|ToString(Integer) (Variables|Default|GetNumberInRing)) " | Side: " (Utilities|String|ToString(Integer) (Variables|Default|GetSide))))
  ;[0.09975 0.798 0 0.5] Spawn a path on clicking center tile
  (if (Actor|ActorHasTag self "Origin")
    (Game|SpawnActorfromClass "/Game/WorldGen/BP_PathNewDefault.BP_PathNewDefault_C" (Math|Transform|MakeTransform "0, 0, 0") "Undefined" "MultiplyWithRoot" 0 0)))

(event EventBeginPlay
  (Variables|Default|SetBaseMat (Rendering|Material|GetMaterial (Variables|Default|GetStaticMesh) 0)))

(event EventOnHovered
  (params (IsHovered :type Boolean))
  ;[0.7826 0.15 0.7652 0.5] Interactions
  (CallFunction|ToggleBlue IsHovered))

(event EventOnInteracted
  (params (TowerToSpawn :type Actor%20Class%20Reference))
  ;[0.7826 0.15 0.7652 0.5] Interactions
  (if (not (Variables|Default|GetIsTowerSpawned))
    (CallFunction|EventShout)
    (Game|SpawnActorfromClass TowerToSpawn (Transformation|GetWorldTransform (Variables|Default|GetTowerSpawnLocation)) "Undefined" "MultiplyWithRoot" 0 0)
    (Variables|Default|SetIsTowerSpawned true)))

(fn ConstructionScript)

(fn ToggleBlue
  (params (IsVisible :type Boolean))
  (bind _staticmesh (Variables|Default|GetStaticMesh))
  (if IsVisible
    (Rendering|Material|SetMaterial _staticmesh 0 "/Game/Materials/M_Blue.M_Blue")
    (else
      (Rendering|Material|SetMaterial _staticmesh 0 (Variables|Default|GetBaseMat)))))