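; Player camera pawn that handles mouse hover and click interaction with world objects.
; On BeginPlay it gets possessed by player 0, shows the cursor and adds the Enhanced Input mapping context.
; Each tick, a cursor trace tracks HoveredActor and sends BI_Interaction hover on/off messages, clearing only on a miss or another interactable.
; The primary action repeats the trace and sends an interacted message to any hit actor implementing the interface.
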(event Input|EnhancedActionEvents|EnhancedInputActionIA_PrimaryAction
  (params (ActionValue :type Boolean) (ElapsedSeconds :type Float%20%28double-precision%29) (TriggeredSeconds :type Float%20%28double-precision%29) (InputAction :type Input%20Action%20Object%20Reference :default "/Game/Inputs/IA_PrimaryAction.IA_PrimaryAction"))
  (bind _returnvalue (Game|GetPlayerController 0))
  (bind (_hitresult _returnvalue_2) (Game|Player|GetHitResultUnderCursorbyChannel _returnvalue "TraceTypeQuery3" true))
  (bind _hitactor (Collision|BreakHitResult _hitresult))
  ;[0.15 0.9391 0.15 0.5] Interacting with the object
  (if _returnvalue_2
    (if (Utilities|DoesObjectImplementInterface _hitactor "/Game/Interface/BI_Interaction.BI_Interaction_C")
      (Class|BIInteraction|OnInteracted(Message) _hitactor))))

(event EventBeginPlay
  (bind _returnvalue (Game|GetPlayerController 0))
  ;[1 0.15 0.15 0.5] Setting up the player camera
  (Pawn|Possess _returnvalue self)
  (Variables|/Script/Engine.PlayerController|SetbShowMouseCursor _returnvalue true)
  (bind _asbp_player_controller (Utilities|Casting|CastToBP_PlayerController _returnvalue))
  (Input|AddMappingContext (PlayerController|LocalPlayerSubsystems|GetEnhancedInputLocalPlayerSubsystem _asbp_player_controller) "/Game/Inputs/IMC_PlayerInputs.IMC_PlayerInputs" 0 "(bIgnoreAllPressedKeysUntilRelease=True,bForceImmediately=False,bNotifyUserSettings=False)"))

(event EventTick
  (params (DeltaSeconds :type Float%20%28single-precision%29))
  ;[0.15 0.15 0.8696 0.5] Checking for a hover target every frame
  (CallFunction|HoveredActorCheck))

(fn ConstructionScript)

(fn HoveredActorCheck
  (bind _returnvalue (Game|GetPlayerController 0))
  (bind (_hitresult _returnvalue_2) (Game|Player|GetHitResultUnderCursorbyChannel _returnvalue "TraceTypeQuery3" true))
  (bind _hitactor (Collision|BreakHitResult _hitresult))
  ;[0.15 0.8609 0.9043 0.5] Sends the onHover interaction to the object that the cursor is over
  (if _returnvalue_2
    (if (Utilities|DoesObjectImplementInterface _hitactor "/Game/Interface/BI_Interaction.BI_Interaction_C")
      (bind _hoveredactor (Variables|Default|GetHoveredActor)
        (:then
          (if (!= _hoveredactor _hitactor)
            (Class|BIInteraction|OnHovered(Message) _hoveredactor false)
            (Variables|Default|SetHoveredActor 0)
            (Variables|Default|SetHoveredActor _hitactor :!label _label)
            (Class|BIInteraction|OnHovered(Message) _hitactor true)))
        (:else
          (goto _label))))
    (else
      (bind _hoveredactor_2 (Variables|Default|GetHoveredActor)
        (:then
          (Class|BIInteraction|OnHovered(Message) _hoveredactor_2 false)
          (Variables|Default|SetHoveredActor 0))
        (:else)))))