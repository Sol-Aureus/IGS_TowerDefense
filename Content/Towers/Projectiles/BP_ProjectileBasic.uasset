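; BP_ProjectileBasic is a basic tower projectile that homes in on a HomingTarget.
; BeginPlay configures its ProjectileMovement for strong homing scaled to InitialSpeed, starts a looping hit-check timer and sets a lifetime limit.
; CheckForHits sphere-traces between the previous and current positions to cover the path travelled.
; It then destroys the actor without using the trace result, so the first check ends the projectile and no damage is applied.
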(event EventBeginPlay
  (bind _initial_speed (Variables|Default|GetInitial%20Speed))
  (bind _returnvalue (Math|Conversions|ToFloat(Integer) _initial_speed))
  (Variables|/Script/Engine.ProjectileMovementComponent|SetHomingTargetComponent (Variables|Default|GetProjectileMovement) (Variables|Default|GetHomingTarget))
  (Variables|/Script/Engine.ProjectileMovementComponent|SetInitialSpeed (Variables|Default|GetProjectileMovement) _returnvalue)
  (Variables|/Script/Engine.ProjectileMovementComponent|SetMaxSpeed (Variables|Default|GetProjectileMovement) _returnvalue)
  (Variables|/Script/Engine.ProjectileMovementComponent|SetHomingAccelerationMagnitude (Variables|Default|GetProjectileMovement) (* _initial_speed 1e+02))
  (Variables|Default|SetCurrentPos (Transformation|GetActorLocation))
  (Utilities|Time|SetTimerbyFunctionName 0 "CheckForHits" 0.1 true true)
  (Utilities|FlowControl|Delay 6.0)
  (Actor|DestroyActor))

(fn ConstructionScript)

(fn CheckforHits
  (bind _output_get (Variables|Default|SetPreviousPos (Variables|Default|GetCurrentPos)))
  (bind _output_get_2 (Variables|Default|SetCurrentPos (Transformation|GetActorLocation)))
  (bind _outhit (Collision|SphereTraceByChannel _output_get _output_get_2 (Variables|Default|GetProjectileRadius) "TraceTypeQuery4" false 0 "None"))
  (Actor|DestroyActor))