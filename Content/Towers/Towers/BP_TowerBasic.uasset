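; BP_TowerBasic is a tower that automatically fires homing projectiles at targets within range.
; A looping timer runs a sphere trace around the tower, keeping the last hit component as the target.
; SpawnProjectile yaws the tower toward it and spawns BP_ProjectileBasic using the attributes' speed and damage.
; Each successful trace pauses the timer for a cooldown derived from attack rate.
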(event Custom|Event_StartAttackTimer
  ;[0.15 0.8609 0.15 0.5] Starting the tower
  (bind _returnvalue (Utilities|Time|SetTimerbyFunctionName 0 "Attack" 0.2 true true))
  (Variables|Default|SetAttackTimer _returnvalue))

(event Custom|Event_StartCooldown
  ;[0.15 0.04651 0.05562 0.5] Cooldown for the attack
  (Utilities|Time|PauseTimerbyHandle (Variables|Default|GetAttackTimer))
  (Utilities|FlowControl|Delay (/ 1.0 (Variables|/Game/Blueprints/BlueprintComponets/BPC_Attributes.BPC_Attributes_C|GetAttackRate (Variables|Default|GetBP_Attributes))))
  (Utilities|Time|UnpauseTimerbyHandle (Variables|Default|GetAttackTimer)))

(event EventBeginPlay
  ;[0.15 0.8609 0.15 0.5] Starting the tower
  (CallFunction|EventStartAttackTimer))

(fn ConstructionScript)

(fn Attack
  (bind _returnvalue (Transformation|GetActorLocation))
  (bind (_outhits _returnvalue_2) (Collision|MultiSphereTraceByChannel _returnvalue _returnvalue (Math|Conversions|ToFloat(Integer) (Variables|/Game/Blueprints/BlueprintComponets/BPC_Attributes.BPC_Attributes_C|GetRange (Variables|Default|GetBP_Attributes))) "TraceTypeQuery4" false 0 "ForDuration" true "(R=1.000000,G=0.000000,B=0.000000,A=1.000000)" "(R=0.000000,G=1.000000,B=0.000000,A=1.000000)" 0.2))
  (if _returnvalue_2
    (CallFunction|EventStartCooldown)
    (for _array_element _outhits
      (Variables|Default|SetHit%20Component (.HitComponent (Collision|BreakHitResult _array_element))))
    (CallFunction|SpawnProjectile)))

(fn SpawnProjectile
  (bind _bp_attributes (Variables|Default|GetBP_Attributes))
  (Transformation|SetActorRotation (Math|Rotator|MakeRotator 0.0 0.0 (.yaw (Math|Rotator|FindLookatRotation (Transformation|GetActorLocation) (Transformation|GetWorldLocation (Variables|Default|GetHit%20Component))))) true)
  (Game|SpawnActorfromClass "/Game/Towers/Projectiles/BP_ProjectileBasic.BP_ProjectileBasic_C" (Transformation|GetActorTransform) "Undefined" "MultiplyWithRoot" 0 (Variables|Default|GetHit%20Component) (Variables|/Game/Blueprints/BlueprintComponets/BPC_Attributes.BPC_Attributes_C|GetProjectileSpeed _bp_attributes) (Variables|/Game/Blueprints/BlueprintComponets/BPC_Attributes.BPC_Attributes_C|GetDamage _bp_attributes) 0))