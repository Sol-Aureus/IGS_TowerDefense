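; Hex grid generator that, on BeginPlay, spawns concentric rings of BP_HexDefault tiles around one already placed in the level.
; SetHexData takes that tile's transform and mesh bounds to derive horizontal and vertical hex spacing.
; Each ring starts at an offset from the origin, then SpawnNextHex walks six sides, stepping from the last tile and tagging ring, side and index.
; CreateNewHexBoard is an empty stub.
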(event EventBeginPlay
  (bind _originhexlocation (Variables|Default|GetOriginHexLocation))
  (bind (_x _y _z) (Math|Vector|BreakVector _originhexlocation))
  (CallFunction|SetHexData)
  (Variables|Default|SetCurrentRingCounter 1)
  (Variables|Default|SetCurrentSideCounter 1)
  ;[0.708 0 0 0.5] Ring Gen + start point for each gen
  (while (<= (Variables|Default|GetCurrentRingCounter) (Variables|Default|GetNumOfRingsToSpawn))
    (bind _returnvalue (Game|SpawnActorfromClass "/Game/Tiles/BP_HexDefault.BP_HexDefault_C" (Math|Transform|MakeTransform (Math|Vector|MakeVector (+ _x (* (Variables|Default|GetCurrentRingCounter) (Variables|Default|GetHorizShift))) (+ _y (* (- (Variables|Default|GetCurrentRingCounter) 2) (Variables|Default|GetVertShift) -1.0)) _z) "0, 0, 0" (Variables|Default|GetOriginHexScale)) "Undefined" "MultiplyWithRoot" 0 0))
    (bind _output_get (Variables|Default|SetLastHexSpawned _returnvalue))
    (Variables|/Game/Tiles/BP_HexDefault.BP_HexDefault_C|SetRing _output_get (Variables|Default|GetCurrentRingCounter))
    (Variables|Default|SetCurrentHexOnSideCounter 1)
    (Math|Integer|IncrementInt (Variables|Default|GetNumberOfHexesThisRing)
      (:%20%20
        (Math|Integer|IncrementInt (Variables|Default|GetCurrentHexOnSideCounter)
          (:%20%20
            ;[1 0.3592 0 0.5] Spawn rest of sides
            (while (<= (Variables|Default|GetCurrentSideCounter) 6)
              ;[0.898 0.982 0 0.5] Spawn rest of hexes in current side
              (while (<= (Variables|Default|GetCurrentHexOnSideCounter) (Variables|Default|GetCurrentRingCounter))
                (switch int (Variables|Default|GetCurrentSideCounter)
                  (:0
                    (Development|PrintString "ERROR IN  SPAWNING HEXES OF SIDE" true true "(R=0.862000,G=0.000000,B=0.000000,A=1.000000)" 5.0))
                  (:1
                    (CallFunction|SpawnNextHex 0.0 -2.0)
                    (Math|Integer|IncrementInt (Variables|Default|GetCurrentHexOnSideCounter) :!label _label))
                  (:2
                    (CallFunction|SpawnNextHex -1.0 -1.0)
                    (goto _label))
                  (:3
                    (CallFunction|SpawnNextHex -1.0 1.0)
                    (goto _label))
                  (:4
                    (CallFunction|SpawnNextHex 0.0 2.0)
                    (goto _label))
                  (:5
                    (CallFunction|SpawnNextHex 1.0 1.0)
                    (goto _label))
                  (:6
                    (CallFunction|SpawnNextHex 1.0 -1.0)
                    (goto _label))))
              (Math|Integer|IncrementInt (Variables|Default|GetCurrentSideCounter)
                (:%20%20
                  (Variables|Default|SetCurrentHexOnSideCounter 1))))
            (Math|Integer|IncrementInt (Variables|Default|GetCurrentRingCounter)
              (:%20%20
                (Variables|Default|SetCurrentSideCounter 1)
                (Variables|Default|SetNumberOfHexesThisRing 1)))))))))

(fn ConstructionScript)

(fn SetHexData
  (bind _returnvalue (Actor|GetActorOfClass "/Game/Tiles/BP_HexDefault.BP_HexDefault_C"))
  (Variables|Default|SetOriginHexScale (Transformation|GetActorScale3D _returnvalue))
  (Variables|Default|SetOriginHexLocation (Transformation|GetActorLocation _returnvalue))
  (Variables|Default|SetOriginHexRotation (Transformation|GetActorRotation _returnvalue))
  (Development|PrintString (Utilities|String|ToString(Vector) (* (+ (Math|Vector|VectorGetAbs (.Min (Components|StaticMesh|GetLocalBounds (Variables|/Game/Tiles/BP_HexDefault.BP_HexDefault_C|GetStaticMesh _returnvalue)))) (.Max (Components|StaticMesh|GetLocalBounds (Variables|/Game/Tiles/BP_HexDefault.BP_HexDefault_C|GetStaticMesh _returnvalue)))) (Transformation|GetWorldScale (Variables|/Game/Tiles/BP_HexDefault.BP_HexDefault_C|GetStaticMesh _returnvalue)))) true true "(R=0.000000,G=0.660000,B=1.000000,A=1.000000)" 5.0)
  (bind _output_get (Variables|Default|SetHexCenterToVerticeWidth (/ (.X (Math|Vector|BreakVector (* (+ (Math|Vector|VectorGetAbs (.Min (Components|StaticMesh|GetLocalBounds (Variables|/Game/Tiles/BP_HexDefault.BP_HexDefault_C|GetStaticMesh _returnvalue)))) (.Max (Components|StaticMesh|GetLocalBounds (Variables|/Game/Tiles/BP_HexDefault.BP_HexDefault_C|GetStaticMesh _returnvalue)))) (Transformation|GetWorldScale (Variables|/Game/Tiles/BP_HexDefault.BP_HexDefault_C|GetStaticMesh _returnvalue))))) 2.0)))
  (Variables|Default|SetHorizShift (* _output_get 1.5))
  (Variables|Default|SetVertShift (* _output_get (Math|Float|Sqrt 3.0) 0.5)))

(fn SpawnNextHex
  (params (xMult :type Float%20%28double-precision%29) (yMult :type Float%20%28double-precision%29))
  (bind _returnvalue (Game|SpawnActorfromClass "/Game/Tiles/BP_HexDefault.BP_HexDefault_C" (Math|Transform|MakeTransform (Math|Vector|MakeVector (+ (.X (Math|Vector|BreakVector (Transformation|GetActorLocation (Variables|Default|GetLastHexSpawned)))) (* xMult (Variables|Default|GetHorizShift))) (+ (.Y (Math|Vector|BreakVector (Transformation|GetActorLocation (Variables|Default|GetLastHexSpawned)))) (* yMult (Variables|Default|GetVertShift) -1.0)) (.Z (Math|Vector|BreakVector (Transformation|GetActorLocation (Variables|Default|GetLastHexSpawned))))) (Variables|Default|GetOriginHexRotation) (Variables|Default|GetOriginHexScale)) "AlwaysSpawn" "MultiplyWithRoot" 0 0))
  (bind _output_get (Variables|Default|SetLastHexSpawned _returnvalue))
  (Variables|/Game/Tiles/BP_HexDefault.BP_HexDefault_C|SetRing _output_get (Variables|Default|GetCurrentRingCounter))
  (Variables|/Game/Tiles/BP_HexDefault.BP_HexDefault_C|SetNumberInRing _output_get (Variables|Default|GetNumberOfHexesThisRing))
  (Math|Integer|IncrementInt (Variables|Default|GetNumberOfHexesThisRing)
    (:%20%20
      (Variables|/Game/Tiles/BP_HexDefault.BP_HexDefault_C|SetSide _output_get (Variables|Default|GetCurrentSideCounter))
      (return))))

(fn CreateNewHexBoard
  (params (HexRingsCount :type Integer)))