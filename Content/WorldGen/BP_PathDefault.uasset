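; BP_PathDefault is a world-generation actor that gathers candidate hexes for a path on the hex grid.
; On BeginPlay it reads the ring count from the BP_HexGridDefault actor and scans all BP_HexDefault actors.
; Hexes on the outermost ring, whose Ring equals that count, are stored in PotentialHexes.
; A random pick from that list exists but is not connected, so no hex is chosen yet.
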(event EventBeginPlay
  (bind _returnvalue (Actor|GetActorOfClass "/Game/WorldGen/BP_HexGridDefault.BP_HexGridDefault_C"))
  (Variables|Default|SetRingCount (Variables|/Game/WorldGen/BP_HexGridDefault.BP_HexGridDefault_C|GetNumOfRingsToSpawn _returnvalue))
  (bind _outactors (Actor|GetAllActorsOfClass "/Game/Tiles/BP_HexDefault.BP_HexDefault_C"))
  (bind _array_element (Utilities|Array|ForEachLoopwithBreak _outactors)
    (:LoopBody
      (if (== (Variables|Default|GetRingCount) (Variables|/Game/Tiles/BP_HexDefault.BP_HexDefault_C|GetRing _array_element))
        (Utilities|Array|Add (Variables|Default|GetPotentialHexes) _array_element)))))

(fn ConstructionScript)