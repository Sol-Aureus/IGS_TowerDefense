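; World-generation actor that builds a random path of BP_Segment actors from the outer ring of the hex grid to the origin hex.
; On BeginPlay it measures the origin hex, picks an outer-ring start hex, removes three candidates from the pool and spawns an inward-facing segment outside it.
; Segments then chain by trigonometry, each turning 60 degrees toward or away from the origin by ChanceToTakeCorrectPath, until within the origin hex.
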(event Custom|Event_NewPath
  (bind _potentialhexes (Variables|Default|GetPotentialHexes))
  (bind _potentialhexes_2 (Variables|Default|GetPotentialHexes))
  (bind _returnvalue (Utilities|Array|Length _potentialhexes_2))
  ;[0.454 0 0 0.5] Make New Path
  ;;[0.782 0 0 0.5] Find Starting Hex
  (if (< _returnvalue 3)
    (Development|PrintString "NOT ENOUGH HEXES TO SPAWN NEW PATH")
    (else
      (bind _output_get (Variables|Default|SetHexIndexForPath (Math|Random|RandomInteger _returnvalue)))
      (Variables|Default|SetStartHex (Utilities|Array|Get(acopy) (Variables|Default|GetPotentialHexes) _output_get))
      (if (== _output_get 0)
        (Utilities|Array|RemoveIndex _potentialhexes (- (Utilities|Array|Length _potentialhexes) 1))
        (for _index (range 0 1)
          (Utilities|Array|RemoveIndex (Variables|Default|GetPotentialHexes) (Variables|Default|GetHexIndexForPath)))
        (else
          (for _index_2 (range 0 2)
            (Utilities|Array|RemoveIndex (Variables|Default|GetPotentialHexes) (- (Variables|Default|GetHexIndexForPath) 2)))))
      ;;[1 0.8446 0.07 0.5] Find starting vertice
      (switch int (Variables|/Game/Tiles/BP_HexDefault.BP_HexDefault_C|GetSide (Variables|Default|GetStartHex))
        (:0
          (Development|PrintString "Something broke in path gen" true true "(R=0.822000,G=0.000000,B=0.000000,A=1.000000)"))
        (:1
          (Variables|Default|SetDegrees 0.0)
          (bind _firstsegment (CallFunction|SpawnFirstSegment :!label _label))
          ;;[1 0.3592 0 0.5] Spawn rest of the segments
          (Variables|Default|SetPreviousSegment _firstsegment)
          (while (> (Math|Vector|Distance(Vector) (Transformation|GetActorLocation (Variables|Default|GetPreviousSegment)) (Variables|Default|GetOriginHexLocation)) (* (Variables|Default|GetHexCenterToVerticeWidth) 1.1))
            (CallFunction|SpawnNextSegment))
          (Development|PrintString "Path successfully generated" true true "(R=0.028313,G=0.742000,B=0.000000,A=1.000000)"))
        (:2
          (Variables|Default|SetDegrees 6e+01)
          (goto _label))
        (:3
          (Variables|Default|SetDegrees 1.2e+02)
          (goto _label))
        (:4
          (Variables|Default|SetDegrees 1.8e+02)
          (goto _label))
        (:5
          (Variables|Default|SetDegrees 2.4e+02)
          (goto _label))
        (:6
          (Variables|Default|SetDegrees 3e+02)
          (goto _label))))))

(event EventBeginPlay
  (CallFunction|SetHexData)
  (bind _returnvalue (Actor|GetActorOfClass "/Game/WorldGen/BP_HexGridDefault.BP_HexGridDefault_C"))
  (Variables|Default|SetRingCount (Variables|/Game/WorldGen/BP_HexGridDefault.BP_HexGridDefault_C|GetNumOfRingsToSpawn _returnvalue))
  (bind _outactors (Actor|GetAllActorsOfClass "/Game/Tiles/BP_HexDefault.BP_HexDefault_C"))
  ;[0.15 0.15 0.15 0.5] Get all hexes in the ring and add them to list as potential hexes to start a path
  (bind _array_element (Utilities|Array|ForEachLoopwithBreak _outactors)
    (:LoopBody
      (if (== (Variables|Default|GetRingCount) (Variables|/Game/Tiles/BP_HexDefault.BP_HexDefault_C|GetRing _array_element))
        (Utilities|Array|Add (Variables|Default|GetPotentialHexes) _array_element)))
    (:Completed
      (CallFunction|EventNewPath))))

(fn ConstructionScript)

(fn SetHexData
  (bind _outactors (Actor|GetAllActorsOfClasswithTag "/Game/Tiles/BP_HexDefault.BP_HexDefault_C" "Origin"))
  (Variables|Default|SetOriginHexScale (Transformation|GetActorScale3D (Utilities|Array|Get(acopy) _outactors)))
  (Variables|Default|SetOriginHexLocation (Transformation|GetActorLocation (Utilities|Array|Get(acopy) _outactors)))
  (Variables|Default|SetOriginHexRotation (Transformation|GetActorRotation (Utilities|Array|Get(acopy) _outactors)))
  (Development|PrintString (Utilities|String|ToString(Vector) (* (+ (Math|Vector|VectorGetAbs (.Min (Components|StaticMesh|GetLocalBounds (Variables|/Game/Tiles/BP_HexDefault.BP_HexDefault_C|GetStaticMesh (Utilities|Array|Get(acopy) _outactors))))) (.Max (Components|StaticMesh|GetLocalBounds (Variables|/Game/Tiles/BP_HexDefault.BP_HexDefault_C|GetStaticMesh (Utilities|Array|Get(acopy) _outactors))))) (Transformation|GetWorldScale (Variables|/Game/Tiles/BP_HexDefault.BP_HexDefault_C|GetStaticMesh (Utilities|Array|Get(acopy) _outactors))))) true true "(R=0.000000,G=0.660000,B=1.000000,A=1.000000)" 5.0)
  (bind _output_get (Variables|Default|SetHexCenterToVerticeWidth (/ (.X (Math|Vector|BreakVector (* (+ (Math|Vector|VectorGetAbs (.Min (Components|StaticMesh|GetLocalBounds (Variables|/Game/Tiles/BP_HexDefault.BP_HexDefault_C|GetStaticMesh (Utilities|Array|Get(acopy) _outactors))))) (.Max (Components|StaticMesh|GetLocalBounds (Variables|/Game/Tiles/BP_HexDefault.BP_HexDefault_C|GetStaticMesh (Utilities|Array|Get(acopy) _outactors))))) (Transformation|GetWorldScale (Variables|/Game/Tiles/BP_HexDefault.BP_HexDefault_C|GetStaticMesh (Utilities|Array|Get(acopy) _outactors)))))) 2.0)))
  (Variables|Default|SetHorizShift (* _output_get 1.5))
  (Variables|Default|SetVertShift (* _output_get (Math|Float|Sqrt 3.0) 0.5)))

(fn SpawnFirstSegment
  (bind _starthex (Variables|Default|GetStartHex))
  (bind _hexcentertoverticewidth (Variables|Default|GetHexCenterToVerticeWidth))
  (bind _returnvalue (Transformation|GetActorLocation _starthex))
  (bind (_x _y _z) (Math|Vector|BreakVector _returnvalue))
  (Development|PrintString (Utilities|String|Append (Utilities|String|ToString(Integer) (Variables|/Game/Tiles/BP_HexDefault.BP_HexDefault_C|GetSide _starthex)) (Utilities|String|ToString(Vector) _returnvalue)) true true "(R=0.918000,G=0.742855,B=0.000000,A=1.000000)" 1e+01)
  (bind _returnvalue_2 (Game|SpawnActorfromClass "/Game/WorldGen/BP_Segment.BP_Segment_C" (Math|Transform|MakeTransform (Math|Vector|MakeVector (+ _x (* (Math|Trig|Cos(Degrees) (Variables|Default|GetDegrees)) _hexcentertoverticewidth 2.0)) (+ _y (* _hexcentertoverticewidth (Math|Trig|Sin(Degrees) (Variables|Default|GetDegrees)) 2.0)) _z) (Math|Rotator|MakeRotator 0.0 0.0 (+ (Variables|Default|GetDegrees) 1.8e+02)) (Variables|Default|GetOriginHexScale)) "AlwaysSpawn" "MultiplyWithRoot" 0 0))
  (Utilities|Array|Add (Variables|Default|GetSegments) _returnvalue_2)
  (return _returnvalue_2))

(fn SpawnNextSegment
  (bind _hexcentertoverticewidth (Variables|Default|GetHexCenterToVerticeWidth))
  (bind _hexcentertoverticewidth_2 (Variables|Default|GetHexCenterToVerticeWidth))
  (bind _hexcentertoverticewidth_3 (Variables|Default|GetHexCenterToVerticeWidth))
  (bind _originhexlocation (Variables|Default|GetOriginHexLocation))
  ;[0.15 0.15 0.15 0.5] "Traverse" and spawn
  (bind _returnvalue (Game|SpawnActorfromClass "/Game/WorldGen/BP_Segment.BP_Segment_C" (Math|Transform|MakeTransform (Math|Vector|MakeVector (+ (.X (Math|Vector|BreakVector (Transformation|GetActorLocation (Variables|Default|GetPreviousSegment)))) (* (Math|Trig|Cos(Degrees) (.Yaw (Math|Rotator|BreakRotator (Transformation|GetActorRotation (Variables|Default|GetPreviousSegment))))) _hexcentertoverticewidth_2 1.0)) (+ (.Y (Math|Vector|BreakVector (Transformation|GetActorLocation (Variables|Default|GetPreviousSegment)))) (* _hexcentertoverticewidth_2 (Math|Trig|Sin(Degrees) (.Yaw (Math|Rotator|BreakRotator (Transformation|GetActorRotation (Variables|Default|GetPreviousSegment))))) 1.0)) (.Z (Math|Vector|BreakVector (Transformation|GetActorLocation (Variables|Default|GetPreviousSegment))))) (Math|Rotator|MakeRotator 0.0 0.0 (.Yaw (Math|Rotator|BreakRotator (Transformation|GetActorRotation (Variables|Default|GetPreviousSegment))))) (Variables|Default|GetOriginHexScale)) "AlwaysSpawn" "MultiplyWithRoot" 0 0))
  (bind _output_get (Variables|Default|SetPreviousSegment _returnvalue))
  (Math|Float|CompareFloat (Math|Vector|Distance(Vector) (Math|Vector|MakeVector (+ (.X (Math|Vector|BreakVector (.Location (Math|Transform|BreakTransform (Transformation|GetActorTransform _output_get))))) (* (Math|Trig|Cos(Degrees) (+ (.Yaw (Math|Rotator|BreakRotator (.Rotation (Math|Transform|BreakTransform (Transformation|GetActorTransform _output_get))))) 6e+01)) _hexcentertoverticewidth_3 1.0)) (+ (.Y (Math|Vector|BreakVector (.Location (Math|Transform|BreakTransform (Transformation|GetActorTransform _output_get))))) (* _hexcentertoverticewidth_3 (Math|Trig|Sin(Degrees) (+ (.Yaw (Math|Rotator|BreakRotator (.Rotation (Math|Transform|BreakTransform (Transformation|GetActorTransform _output_get))))) 6e+01)) 1.0)) (.Z (Math|Vector|BreakVector (.Location (Math|Transform|BreakTransform (Transformation|GetActorTransform _output_get)))))) _originhexlocation) (Math|Vector|Distance(Vector) (Math|Vector|MakeVector (+ (.X (Math|Vector|BreakVector (.Location (Math|Transform|BreakTransform (Transformation|GetActorTransform _output_get))))) (* (Math|Trig|Cos(Degrees) (- (.Yaw (Math|Rotator|BreakRotator (.Rotation (Math|Transform|BreakTransform (Transformation|GetActorTransform _output_get))))) 6e+01)) _hexcentertoverticewidth 1.0)) (+ (.Y (Math|Vector|BreakVector (.Location (Math|Transform|BreakTransform (Transformation|GetActorTransform _output_get))))) (* _hexcentertoverticewidth (Math|Trig|Sin(Degrees) (- (.Yaw (Math|Rotator|BreakRotator (.Rotation (Math|Transform|BreakTransform (Transformation|GetActorTransform _output_get))))) 6e+01)) 1.0)) (.Z (Math|Vector|BreakVector (.Location (Math|Transform|BreakTransform (Transformation|GetActorTransform _output_get)))))) _originhexlocation)
    (:>
      (LocalVariables|SetFartherDirectionToRotateTo (Math|Rotator|MakeRotator 0.0 0.0 (+ (.Yaw (Math|Rotator|BreakRotator (Transformation|GetActorRotation (Variables|Default|GetPreviousSegment)))) 6e+01)) :!label _label)
      (LocalVariables|SetCloserDirectionToRotateTo (Math|Rotator|MakeRotator 0.0 0.0 (- (.Yaw (Math|Rotator|BreakRotator (Transformation|GetActorRotation (Variables|Default|GetPreviousSegment)))) 6e+01))))
    (:==
      (if (Math|Random|RandomBool)
        (goto _label)
        (else
          (LocalVariables|SetFartherDirectionToRotateTo (Math|Rotator|MakeRotator 0.0 0.0 (- (.Yaw (Math|Rotator|BreakRotator (Transformation|GetActorRotation (Variables|Default|GetPreviousSegment)))) 6e+01)) :!label _label_2)
          (LocalVariables|SetCloserDirectionToRotateTo (Math|Rotator|MakeRotator 0.0 0.0 (+ (.Yaw (Math|Rotator|BreakRotator (Transformation|GetActorRotation (Variables|Default|GetPreviousSegment)))) 6e+01))))))
    (:<
      (goto _label_2)))
  (if (<= (Math|Random|RandomFloat) (Variables|Default|GetChanceToTakeCorrectPath))
    ;[0.15 0.15 0.15 0.5] Rotate segment and add to array
    (Transformation|SetActorRotation (Variables|Default|GetPreviousSegment) (LocalVariables|GetCloserDirectionToRotateTo) true)
    (else
      (Transformation|SetActorRotation (Variables|Default|GetPreviousSegment) (LocalVariables|GetFartherDirectionToRotateTo) true)))
  (Utilities|Array|Add (Variables|Default|GetSegments) (Variables|Default|GetPreviousSegment))
  (return))