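; GM_IGSTowerDefense is a tower defense game mode, apparently an early test of hex tile spacing.
; On BeginPlay, SetCenterToVerticeWidth finds a BP_HexDefault in the level and derives its scaled size from the static mesh's local bounds.
; It prints that size and spawns one more hex at a world position computed from the X extent using half-width and square-root-of-three factors.
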(event EventBeginPlay
  (CallFunction|SetCentertoVerticeWidth))

(event EventTick
  (params (DeltaSeconds :type Float%20%28single-precision%29)))

(fn ConstructionScript)

(fn SetCentertoVerticeWidth
  (bind _returnvalue (Actor|GetActorOfClass "/Game/Tiles/BP_HexDefault.BP_HexDefault_C"))
  (Development|PrintString (Utilities|String|ToString(Vector) (* (+ (Math|Vector|VectorGetAbs (.Min (Components|StaticMesh|GetLocalBounds (Variables|/Game/Tiles/BP_HexDefault.BP_HexDefault_C|GetStaticMesh _returnvalue)))) (.Max (Components|StaticMesh|GetLocalBounds (Variables|/Game/Tiles/BP_HexDefault.BP_HexDefault_C|GetStaticMesh _returnvalue)))) (Transformation|GetWorldScale (Variables|/Game/Tiles/BP_HexDefault.BP_HexDefault_C|GetStaticMesh _returnvalue)))) true true "(R=0.000000,G=0.660000,B=1.000000,A=1.000000)" 5.0)
  (Game|SpawnActorfromClass "/Game/Tiles/BP_HexDefault.BP_HexDefault_C" (Math|Transform|MakeTransform (Math|Vector|MakeVector (* (.X (Math|Vector|BreakVector (* (+ (Math|Vector|VectorGetAbs (.Min (Components|StaticMesh|GetLocalBounds (Variables|/Game/Tiles/BP_HexDefault.BP_HexDefault_C|GetStaticMesh _returnvalue)))) (.Max (Components|StaticMesh|GetLocalBounds (Variables|/Game/Tiles/BP_HexDefault.BP_HexDefault_C|GetStaticMesh _returnvalue)))) (Transformation|GetWorldScale (Variables|/Game/Tiles/BP_HexDefault.BP_HexDefault_C|GetStaticMesh _returnvalue))))) 0.5) (* (.X (Math|Vector|BreakVector (* (+ (Math|Vector|VectorGetAbs (.Min (Components|StaticMesh|GetLocalBounds (Variables|/Game/Tiles/BP_HexDefault.BP_HexDefault_C|GetStaticMesh _returnvalue)))) (.Max (Components|StaticMesh|GetLocalBounds (Variables|/Game/Tiles/BP_HexDefault.BP_HexDefault_C|GetStaticMesh _returnvalue)))) (Transformation|GetWorldScale (Variables|/Game/Tiles/BP_HexDefault.BP_HexDefault_C|GetStaticMesh _returnvalue))))) (Math|Float|Sqrt 3.0)) 0.0) "0.000000,0.000000,0.000000") "Undefined" "MultiplyWithRoot" 0 0))