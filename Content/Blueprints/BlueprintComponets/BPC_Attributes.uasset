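; BPC_Attributes is an actor component that stores a set of combat and movement stats such as health, damage, range, attack rate and speeds.
; ChangeAttribute switches on an attribute selector and adds the given delta to the matching stat.
; Most stats are truncated to integers after the change, while Attack Rate and Stop Time keep fractional values.
; It applies no clamping, and BeginPlay is unused.
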(event EventBeginPlay)

(fn ChangeAttribute
  (params (AttributeToChange :type E_Attributes%20Enum :default "NewEnumerator0") (ChangeValue :type Float%20%28double-precision%29))
  (switch Utilities|FlowControl|Switch|SwitchonE_Attributes AttributeToChange
    (:NewEnumerator0
      (Variables|Default|SetHealth (Math|Float|Truncate (+ (Variables|Default|GetHealth) ChangeValue))))
    (:NewEnumerator1
      (Variables|Default|SetDamage (Math|Float|Truncate (+ (Variables|Default|GetDamage) ChangeValue))))
    (:NewEnumerator2
      (Variables|Default|SetRange (Math|Float|Truncate (+ (Variables|Default|GetRange) ChangeValue))))
    (:NewEnumerator3
      (Variables|Default|SetAttackRate (+ (Variables|Default|GetAttackRate) ChangeValue)))
    (:NewEnumerator4
      (Variables|Default|SetStopTime (+ (Variables|Default|GetStopTime) ChangeValue)))
    (:NewEnumerator5
      (Variables|Default|SetMoveSpeed (Math|Float|Truncate (+ (Variables|Default|GetMoveSpeed) ChangeValue))))
    (:NewEnumerator6
      (Variables|Default|SetProjectileSpeed (Math|Float|Truncate (+ (Variables|Default|GetProjectileSpeed) ChangeValue))))))