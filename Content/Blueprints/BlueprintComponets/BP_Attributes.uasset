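; BP_Attributes is a component Blueprint that holds combat and movement stats, including health, damage, range, attack rate, stop time, move speed and projectile speed.
; Each stat has a plain setter and getter with no clamping, validation or change notification.
; Its event graph is empty, so it acts purely as a data container for other Blueprints to read and write.
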(event EventBeginPlay)

(event EventTick
  (params (DeltaSeconds :type Float%20%28single-precision%29)))

(fn SetHealth
  (params (NewHealth :type Integer))
  (Variables|Default|SetHealth NewHealth))

(fn SetDamage
  (params (NewDamage :type Integer))
  (Variables|Default|SetDamage NewDamage))

(fn SetRange
  (params (NewRange :type Integer))
  (Variables|Default|SetRange NewRange))

(fn SetAttackRate
  (params (NewAttackRate :type Float%20%28double-precision%29))
  (Variables|Default|SetAttackRate NewAttackRate))

(fn SetStopTime
  (params (NewStopTime :type Float%20%28double-precision%29))
  (Variables|Default|SetStopTime NewStopTime))

(fn SetMoveSpeed
  (params (NewMoveSpeed :type Integer))
  (Variables|Default|SetMoveSpeed NewMoveSpeed))

(fn SetProjectileSpeed
  (params (NewProjectileSpeed :type Integer))
  (Variables|Default|SetProjectileSpeed NewProjectileSpeed))

(fn GetHealth
  (return (Variables|Default|GetHealth)))

(fn GetDamage
  (return (Variables|Default|GetDamage)))

(fn GetRange
  (return (Variables|Default|GetRange)))

(fn GetAttackRate
  (return (Variables|Default|GetAttackRate)))

(fn GetStopTime
  (return (Variables|Default|GetStopTime)))

(fn GetMoveSpeed
  (return (Variables|Default|GetMoveSpeed)))

(fn GetProjectileSpeed
  (return (Variables|Default|GetProjectileSpeed)))